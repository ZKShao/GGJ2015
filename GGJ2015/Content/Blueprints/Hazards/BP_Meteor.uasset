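; BP_Meteor is a hazard actor that moves along its Velocity and explodes when it hits something.
; Tick moves it with a swept world offset.
; On Hit, it damages pawns found by a sphere overlap around the impact point, spawns ten explosion emitters at that same point with auto-destroy off, then destroys itself.
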(event `self.ReceiveTick`
  (params (DeltaSeconds :type "Float (single-precision)"))
  (`self.K2_AddActorWorldOffset` (* (`self.Velocity`) DeltaSeconds) true))

(event `self.ReceiveHit`
  (params (MyComp :type "PrimitiveComponent Object Reference") (Other :type "Actor Object Reference") (OtherComp :type "PrimitiveComponent Object Reference") (bSelfMoved :type Boolean) (HitLocation :type "Object.Vector Structure") (HitNormal :type "Object.Vector Structure") (NormalImpulse :type "Object.Vector Structure") (Hit :type "EngineTypes.HitResult Structure (by ref)"))
  (`|ExecutionSequence`
    (:`then_0`
      (bind _outactors (`KismetSystemLibrary.SphereOverlapActors_NEW` HitLocation 200.0 (`|MakeArray` "ObjectTypeQuery3" :!type "EngineTypes.EObjectTypeQuery Enum")))
      (for _array_element _outactors
        (`GameplayStatics.ApplyDamage` _array_element 100.0)))
    (:`then_1`
      (for _ (range 10)
        (`GameplayStatics.SpawnEmitterAtLocation` "/Game/StarterContent/Particles/P_Explosion.P_Explosion" (+ HitLocation (0.0 0.0 0.0)) (struct) false)))
    (:`then_2`
      (`self.K2_DestroyActor`))))

(fn `UserConstructionScript`)