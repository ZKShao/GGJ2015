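; BP_GhostGenerator is a Blueprint that, despite its name, holds only the end-of-run score display and return to the main menu.
; Its ShowScore event creates a ScoreScreen widget from a time in seconds and before and after player counts, then switches the first player controller to UI-only input.
; After a fixed delay it removes the widget and opens the Main Menu level.
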(event `self.BP_ShowScore`
  (params (Time :type Integer) (NumBefore :type Integer) (NumAfter :type Integer))
  (bind _returnvalue (`GameplayStatics.GetPlayerController` 0))
  (bind _returnvalue_2 (`|CreateWidget` "/Game/Blueprints/UMG/ScoreScreen.ScoreScreen_C" _returnvalue (`KismetTextLibrary.Conv_StringToText` (`KismetStringLibrary.BuildString_Int` "" "" Time " seconds")) (`KismetTextLibrary.Conv_StringToText` (`KismetStringLibrary.BuildString_Int` "" "" NumBefore " players")) (`KismetTextLibrary.Conv_StringToText` (`KismetStringLibrary.BuildString_Int` "" "" NumAfter " players"))))
  (`WidgetBlueprintLibrary.SetInputMode_UIOnlyEx` _returnvalue _returnvalue_2)
  (set `self.ScoreWidget` _returnvalue_2)
  (`UserWidget.AddToViewport` _returnvalue_2)
  (`KismetSystemLibrary.Delay` 5.0)
  (`Widget.RemoveFromParent` (`self.ScoreWidget`))
  (`GameplayStatics.OpenLevel` "Main Menu"))

(fn `UserConstructionScript`)