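; BP_GhostCharacter is a ghost character that shows its name on a floating text label.
; On init the label text is set to the given name, and each tick it is rotated from the player camera's rotation, turned 180 degrees to face the view.
; Ghost events are only printed by enum name as debug output.
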(event `self.ReceiveTick`
  (params (DeltaSeconds :type "Float (single-precision)"))
  (`SceneComponent.K2_SetWorldRotation` (`self.TextRender1`) (`KismetMathLibrary.ComposeRotators` (struct :`Yaw` 180.0) (`PlayerCameraManager.GetCameraRotation` (`GameplayStatics.GetPlayerCameraManager` 0))) false))

(event `self.OnGhostInit`
  (params (Name :type String) (RemainingTime :type "Float (single-precision)"))
  (`TextRenderComponent.SetText` (`self.TextRender1`) Name))

(event `self.OnGhostEvent`
  (params (Event :type "EGhostEvent Enum" :default "Jump"))
  (`KismetSystemLibrary.PrintString` (`|GetEnumeratorNameAsString` Event)))

(fn `UserConstructionScript`)