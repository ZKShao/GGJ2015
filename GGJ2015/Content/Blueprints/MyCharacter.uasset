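; Player character Blueprint with world-axis movement, jumping and a toggle between its own view and a map camera.
; On BeginPlay it caches the first BP_Camera found in the level as MapCamera.
; Move inputs push along fixed world X and Y, independent of camera or control rotation.
; ToggleCamera flips a flag and switches player 0's view target between MapCamera and the character, provided a map camera exists.
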(event `self.ReceiveBeginPlay`
  (bind _outactors (`GameplayStatics.GetAllActorsOfClass` "/Game/Blueprints/BP_Camera.BP_Camera_C"))
  (if (> (`KismetArrayLibrary.Array_Length` _outactors) 0)
    (set `self.MapCamera` (`KismetArrayLibrary.Array_Get` _outactors))))

(event `InputAxis|MoveForward`
  (params (AxisValue :type "Float (single-precision)"))
  ;[1 1 1] movement
  (`self.AddMovementInput` (1.0 0.0 0.0) AxisValue))

(event `InputAxis|MoveRight`
  (params (AxisValue :type "Float (single-precision)"))
  ;[1 1 1] movement
  (`self.AddMovementInput` (0.0 1.0 0.0) AxisValue))

(event `InputAction|ToggleCamera`
  ;[1 1 1] movement
  (:`Pressed`
    (`self.ToggleMapCamera`)))

(event `InputAction|Junp`
  ;[1 1 1] movement
  (:`Pressed`
    (if (`self.CanJump`)
      (`self.Jump`)))
  (:`Released`
    (`self.StopJumping`)))

(fn `ToggleMapCamera`
  (bind _returnvalue (`GameplayStatics.GetPlayerController` 0))
  (if (!= (`self.MapCamera`) null)
    (set `self.ViewingMapCamera` (not (`self.ViewingMapCamera`)))
    (if (`self.ViewingMapCamera`)
      (`PlayerController.SetViewTargetWithBlend` _returnvalue (`self.MapCamera`) 0.0 "VTBlend_Linear" 0.0 false)
      (else
        (`PlayerController.SetViewTargetWithBlend` _returnvalue self 0.0 "VTBlend_Linear" 0.0 false)))))

(fn `UserConstructionScript`)