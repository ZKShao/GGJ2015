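; Player Paper2D character with walk, jump and dash along world X/Y, plus a Tab toggle to view a map camera.
; Tick derives facing from velocity, with Y overriding X, then picks placeholder idle, dash, walk or jump flipbooks, using CanJump to separate walking from jumping.
; Dash boosts velocity and max walk speed, with named timers ending the burst and the cooldown.
; The map view switches view target to the first BP_Camera found at BeginPlay.
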(event `self.ReceiveBeginPlay`
  (bind _outactors (`GameplayStatics.GetAllActorsOfClass` "/Game/Blueprints/BP_Camera.BP_Camera_C"))
  (if (> (`KismetArrayLibrary.Array_Length` _outactors) 0)
    (set `self.MapCamera` (`KismetArrayLibrary.Array_Get` _outactors))))

(event `Key|Tab`
  (:`Pressed`
    (`self.ToggleMapCamera`)))

(event `InputAxis|Horizontal`
  (params (AxisValue :type "Float (single-precision)"))
  ;[1 1 1] Input
  (`self.AddMovementInput` (1.0 0.0 0.0) AxisValue))

(event `self.ReceiveTick`
  (params (DeltaSeconds :type "Float (single-precision)"))
  (bind _sprite (`self.Sprite`))
  (bind _sprite_2 (`self.Sprite`))
  (bind _sprite_3 (`self.Sprite`))
  (`/Engine/EditorBlueprintResources/StandardMacros.CompareFloat` (.x (`MovementComponent.Velocity` (`self.CharacterMovement`)))
    (:`>`
      (set `self.Facing` "R"))
    (:`==`
      (set `self.Facing` "Idle"))
    (:`<`
      (set `self.Facing` "L")))
  (`/Engine/EditorBlueprintResources/StandardMacros.CompareFloat` (.y (`MovementComponent.Velocity` (`self.CharacterMovement`)))
    (:`>`
      (set `self.Facing` "D"))
    (:`==`
      _)
    (:`<`
      (set `self.Facing` "U")))
  (if (`KismetStringLibrary.EqualEqual_StrStr` (`self.Facing`) "Idle")
    (`PaperFlipbookComponent.SetFlipbook` (`self.Sprite`) "/Game/Animations/Placeholders/Idle_placeholder_Flipbook.Idle_placeholder_Flipbook")
    (elif (`self.isDashing`)
      (switch `string` (`self.Facing`)
        (:`U`
          (`PaperFlipbookComponent.SetFlipbook` _sprite_2 "/Game/Animations/Placeholders/Dash_U_placeholder_Flipbook.Dash_U_placeholder_Flipbook"))
        (:`D`
          (`PaperFlipbookComponent.SetFlipbook` _sprite_2 "/Game/Animations/Placeholders/Dash_D_placeholder_Flipbook.Dash_D_placeholder_Flipbook"))
        (:`L`
          (`PaperFlipbookComponent.SetFlipbook` _sprite_2 "/Game/Animations/Placeholders/Dash_L_placeholder_Flipbook.Dash_L_placeholder_Flipbook"))
        (:`R`
          (`PaperFlipbookComponent.SetFlipbook` _sprite_2 "/Game/Animations/Placeholders/Dash_R_placeholder_Flipbook.Dash_R_placeholder_Flipbook")))
      (elif (`self.CanJump`)
        (switch `string` (`self.Facing`)
          (:`U`
            (`PaperFlipbookComponent.SetFlipbook` _sprite_3 "/Game/Animations/Placeholders/Walk_U_placeholder_Flipbook.Walk_U_placeholder_Flipbook"))
          (:`D`
            (`PaperFlipbookComponent.SetFlipbook` _sprite_3 "/Game/Animations/Placeholders/Walk_D_Placeholder_Flipbook.Walk_D_Placeholder_Flipbook"))
          (:`L`
            (`PaperFlipbookComponent.SetFlipbook` _sprite_3 "/Game/Animations/Placeholders/Walk_L_placeholder_Flipbook.Walk_L_placeholder_Flipbook"))
          (:`R`
            (`PaperFlipbookComponent.SetFlipbook` _sprite_3 "/Game/Animations/Placeholders/Walk_R_placeholder_Flipbook.Walk_R_placeholder_Flipbook")))
        (else
          (switch `string` (`self.Facing`)
            (:`U`
              (`PaperFlipbookComponent.SetFlipbook` _sprite "/Game/Animations/Placeholders/Jump_U_placeholder_Flipbook.Jump_U_placeholder_Flipbook"))
            (:`D`
              (`PaperFlipbookComponent.SetFlipbook` _sprite "/Game/Animations/Placeholders/Jump_D_placeholder_Flipbook.Jump_D_placeholder_Flipbook"))
            (:`L`
              (`PaperFlipbookComponent.SetFlipbook` _sprite "/Game/Animations/Placeholders/Jump_L_placeholder_Flipbook.Jump_L_placeholder_Flipbook"))
            (:`R`
              (`PaperFlipbookComponent.SetFlipbook` _sprite "/Game/Animations/Placeholders/Jump_R_placeholder_Flipbook.Jump_R_placeholder_Flipbook"))))))))

(event `InputAxis|Vertical`
  (params (AxisValue :type "Float (single-precision)"))
  ;[1 1 1] Input
  (`self.AddMovementInput` (0.0 -1.0 0.0) AxisValue))

(event `InputAction|Dash`
  (bind _charactermovement (`self.CharacterMovement`))
  ;[1 1 1] Input
  (:`Pressed`
    (if (`self.canDash`)
      (set `self.canDash` false)
      (set `self.isDashing` true)
      (set `CharacterMovementComponent.MaxWalkSpeed` 1500.0 _charactermovement)
      (set `MovementComponent.Velocity` (* (`KismetMathLibrary.Normal` (`MovementComponent.Velocity` _charactermovement)) 1500.0) _charactermovement)
      (`KismetSystemLibrary.K2_SetTimer` null "DashDone" 0.3)
      (`KismetSystemLibrary.K2_SetTimer` null "DashCooledDown" 1.3))))

(event `InputAction|Jump`
  ;[1 1 1] Input
  (:`Pressed`
    (if (`self.CanJump`)
      (`self.Jump`)))
  (:`Released`
    (`self.StopJumping`)))

(fn `DashCooledDown`
  (set `self.canDash` true))

(fn `DashDone`
  (set `CharacterMovementComponent.MaxWalkSpeed` 600.0 (`self.CharacterMovement`))
  (set `self.isDashing` false))

(fn `ToggleMapCamera`
  (bind _returnvalue (`GameplayStatics.GetPlayerController` 0))
  (bind _viewingmapcamera (`self.ViewingMapCamera`))
  (if (!= (`self.MapCamera`) null)
    (set `self.ViewingMapCamera` (not _viewingmapcamera))
    (if _viewingmapcamera
      (`PlayerController.SetViewTargetWithBlend` _returnvalue (`self.MapCamera`) 0.0 "VTBlend_Linear" 0.0 false)
      (else
        (`PlayerController.SetViewTargetWithBlend` _returnvalue self 0.0 "VTBlend_Linear" 0.0 false)))))

(fn `UserConstructionScript`
  (set `self.canDash` true))